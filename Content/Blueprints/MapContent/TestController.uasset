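; Test controller for a tile-based map that spawns units and handles tile selection, using the map grid and unit types from TileBasedGameMode.
; Pressing E spawns a random unit on a random empty grid tile by shuffling both lists, then registers it on that tile.
; Selection swaps the selected tile and toggles its UI, then arranges any occupying unit's squads and calls CallPathfinder, which is an empty stub.
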(event `self.ReceiveBeginPlay`
  (bind _astile_based_game_mode (cast `/Game/Blueprints/TileBasedGameMode` (`GameplayStatics.GetGameMode`))
    (:`then`
      (set `self.TheGameMode` _astile_based_game_mode))
    (:`CastFailed`
      (`KismetSystemLibrary.PrintString` "wrong GameMode"))))

(event `Key|E`
  (params (Key :type "Key Structure" :default "AnyKey"))
  (:`Pressed`
    (`self.SpawnRandomUnit`)))

(fn `CallPathfinder`
  (params (Unit :type "/Game/Blueprints/MapContent/BasicUnit Object Reference") (StartTile :type "/Game/Blueprints/MapContent/BasicTile Object Reference")))

(fn `Selection`
  (params (Selected :type "/Game/Blueprints/MapContent/BasicTile Object Reference"))
  (bind _selectedtile (`self.SelectedTile`))
  (bind _item (`KismetArrayLibrary.Array_Get` (`self.SelectedTile`)))
  (for _array_element _selectedtile
    (`SceneComponent.ToggleVisibility` (`/Game/Blueprints/MapContent/BasicTile.SelectUI` _array_element) false))
  (`KismetArrayLibrary.Array_Clear` _selectedtile)
  (`KismetArrayLibrary.Array_Add` _selectedtile Selected)
  (`SceneComponent.ToggleVisibility` (`/Game/Blueprints/MapContent/BasicTile.SelectUI` Selected) false)
  (bind (_unit _isempty) (`/Game/Blueprints/MapContent/BasicTile.curUnitOrEmpty` _item))
  (if (not _isempty)
    (`/Game/Blueprints/MapContent/BasicUnit.ArrangeSquads` _unit)
    (`self.CallPathfinder` _unit _item)))

(fn `SpawnRandomUnit`
  (bind _thegamemode (`self.TheGameMode`))
  (bind _unittypes (`/Game/Blueprints/TileBasedGameMode.UnitTypes` _thegamemode))
  (bind _availabletiles (`/Game/Blueprints/MapContent/BP_MapGrid.getEmptyTiles` (`/Game/Blueprints/TileBasedGameMode.MapGridReference` _thegamemode)))
  (`KismetArrayLibrary.Array_Shuffle` _availabletiles)
  (`KismetArrayLibrary.Array_Shuffle` _unittypes)
  (bind _item (`KismetArrayLibrary.Array_Get` _availabletiles))
  (bind _returnvalue (`|SpawnActorFromClass` (`GameplayStatics.GetObjectClass` (`KismetArrayLibrary.Array_Get` _unittypes)) (`self.GetTransform` _item) "AlwaysSpawn" "OverrideRootScale"))
  (`/Game/Blueprints/MapContent/BasicTile.setUnit` _item _returnvalue)
  (bind (_unit _isempty) (`/Game/Blueprints/MapContent/BasicTile.curUnitOrEmpty` _item))
  (`KismetSystemLibrary.PrintString` (`KismetStringLibrary.Conv_BoolToString` _isempty)))

(fn `UserConstructionScript`)