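; BP_MapGrid is an actor that builds and queries the tile map for a tile-based game, using map size and tile types from TileBasedGameMode.
; ConstructGrid spawns a random tile type at each converted grid position, sets its coordinates and stores it in AllTiles.
; GetTileAt looks tiles up by flattened X/Y index, and GetEmptyTiles rebuilds and returns the list of unoccupied tiles.
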(event `self.ReceiveBeginPlay`
  (bind _astile_based_game_mode (cast `/Game/Blueprints/TileBasedGameMode` (`GameplayStatics.GetGameMode`))
    (:`then`
      (set `self.GameMode` _astile_based_game_mode))
    (:`CastFailed`
      (`KismetSystemLibrary.PrintString` "BP_MapGrid: Cast to TileBasedGameMode failed"))))

(fn `constructGrid`
  (bind _gamemode (`self.GameMode`))
  (bind _tiletypes (`/Game/Blueprints/TileBasedGameMode.TileTypes` (`self.GameMode`)))
  ;[1 1 1] MapSize Dimensions
  (set `self.MapSize_X` (`/Game/Blueprints/TileBasedGameMode.MapSize_X` _gamemode))
  (set `self.MapSize_Y` (`/Game/Blueprints/TileBasedGameMode.MapSize_Y` _gamemode))
  (for _index (range (`self.MapSize_X`))
    (for _index_2 (range (`self.MapSize_Y`))
      (bind _xy (`/Game/Blueprints/TileBasedGameMode.convertPosition` (`self.GameMode`) _index _index_2 0))
      ;[1 1 1] Spawn Tile, set IntegerPosition and Array for easier search later
      (bind _returnvalue (`|SpawnActorFromClass` (`KismetArrayLibrary.Array_Get` _tiletypes (`KismetMathLibrary.RandomIntegerInRange` 0 (`KismetArrayLibrary.Array_LastIndex` _tiletypes))) _xy "AlwaysSpawn" "OverrideRootScale" self))
      (`/Game/Blueprints/MapContent/BasicTile.SetCoordinates` _returnvalue _index _index_2)
      (`KismetArrayLibrary.Array_Add` (`self.AllTiles`) _returnvalue))))

(fn `getEmptyTiles`
  (returns (AvailableTiles :type "Array of /Game/Blueprints/MapContent/BasicTile Object Reference"))
  (bind _emptytiles (`self.EmptyTiles`))
  ;[1 1 1] Check allTiles if Occupied or Empty
  (`KismetArrayLibrary.Array_Clear` _emptytiles)
  (for _array_element (`self.AllTiles`)
    (bind _asbasic_tile (cast `/Game/Blueprints/MapContent/BasicTile` _array_element)
      (:`then`
        (bind (_unit _isempty) (`/Game/Blueprints/MapContent/BasicTile.curUnitOrEmpty` _asbasic_tile))
        (if _isempty
          (`KismetArrayLibrary.Array_Add` _emptytiles _asbasic_tile)))
      (:`CastFailed`
        (`KismetSystemLibrary.PrintString` "GetAvailableSpace:cast to basic Tile failed"))))
  (return _emptytiles))

(fn `getTileAt`
  (params (X :type Integer) (Y :type Integer))
  (returns (Item :type "Actor Object Reference"))
  (return (`KismetArrayLibrary.Array_Get` (`self.AllTiles`) (+ (* (`/Game/Blueprints/TileBasedGameMode.MapSize_Y` (`self.GameMode`)) X) Y))))

(fn `UserConstructionScript`)