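; BasicTile is a map tile that stores X/Y coordinates and tracks the unit placed on it.
; SetUnit appends to the CurUnit array and ClearTile empties it.
; GetCurUnit reads only the first entry, returning it as a BasicUnit or reporting the tile empty if the cast fails.
; Its event graph and construction script have no logic, so state changes only through these functions.
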(event `self.ReceiveBeginPlay`)

(event `self.ReceiveTick`
  (params (DeltaSeconds :type "Float (single-precision)")))

(fn `clearTile`
  (`KismetArrayLibrary.Array_Clear` (`self.curUnit`)))

(fn `getCurUnit`
  (returns (Unit :type "/Game/Blueprints/MapContent/BasicUnit Object Reference") (isEmpty :type Boolean))
  (bind _asbasic_unit (cast `/Game/Blueprints/MapContent/BasicUnit` (`KismetArrayLibrary.Array_Get` (`self.curUnit`)))
    (:`then`
      (return _asbasic_unit false))
    (:`CastFailed`
      (return null true))))

(fn `SetCoordinates`
  (params (_X :type Integer) (_Y :type Integer))
  (set `self._X` _X)
  (set `self._Y` _Y))

(fn `setUnit`
  (params (NewUnit :type "/Game/Blueprints/MapContent/BasicUnit Object Reference"))
  (`KismetArrayLibrary.Array_Add` (`self.curUnit`) NewUnit))

(fn `UserConstructionScript`)