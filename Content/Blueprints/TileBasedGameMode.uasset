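; Game mode for a tile-based game with units, setting up the map and pathfinder on BeginPlay.
; InitGame records level-placed BasicTile and BasicUnit actors as available types and destroys them, then spawns Pathfinder2 and BP_MapGrid, keeps references, and constructs the grid.
; Helpers linearly search tiles by X/Y for tile and occupant, and convert grid coordinates to scaled world transforms.
; Pathfinding grid update and node display calls are left unconnected.
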(event `self.ReceiveBeginPlay`
  (`self.InitGame`))

(fn `convertPosition`
  (params (X :type Integer) (Y :type Integer))
  (returns (XY :type "Transform Structure"))
  ;[1 1 1] Convert Integer Position to WorldTransform with MapScale
  (return (`self.ConvertWorldTransform` X Y)))

(fn `RegisterContent`
  ;[1 1 1] Add new Tiles and Units to the current level and this will register them for later use
  (bind _outactors (`GameplayStatics.GetAllActorsOfClass` "/Game/Blueprints/MapContent/BasicTile.BasicTile_C"))
  (set `self.TileTypes` _outactors)
  (bind _outactors_2 (`GameplayStatics.GetAllActorsOfClass` "/Game/Blueprints/MapContent/BasicUnit.BasicUnit_C"))
  (set `self.UnitTypes` _outactors_2)
  (for _array_element _outactors
    (`self.K2_DestroyActor` _array_element))
  (for _array_element_2 _outactors_2
    (`self.K2_DestroyActor` _array_element_2)))

(fn `SearchPosition`
  (params (SearchAtX :type Integer) (SearchAtY :type Integer))
  (returns (TileAtPosition :type "/Game/Blueprints/MapContent/BasicTile Object Reference") (UnitAtPosition :type "/Game/Blueprints/MapContent/BasicUnit Object Reference") (IsTileEmpty :type Boolean))
  (for _array_element (`self.AllTiles`)
    (bind _asbasic_tile (cast `/Game/Blueprints/MapContent/BasicTile` _array_element))
    (if (and (== SearchAtX (`/Game/Blueprints/MapContent/BasicTile._X` _asbasic_tile)) (== SearchAtY (`/Game/Blueprints/MapContent/BasicTile._Y` _asbasic_tile)))
      (bind (_unit _isempty) (`/Game/Blueprints/MapContent/BasicTile.curUnitOrEmpty` _asbasic_tile))
      (return _asbasic_tile _unit _isempty))))

(fn `UserConstructionScript`)