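; Pathfinder actor for a tile-based game that mirrors the map with a grid of spawned PathNode actors holding coordinates, move cost and occupancy.
; Helpers look up nodes by coordinate, pick the cheapest by accumulated cost, bounds-check neighbour offsets and show nodes as debug meshes.
; The Dijkstra-style range search is unfinished, with an empty neighbour loop.
; The grid update reads tile info but never applies it.
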(event `self.ReceiveBeginPlay`)

(fn `createPathfindingGrid`
  (bind _astile_based_game_mode (cast `/Game/Blueprints/TileBasedGameMode` (`GameplayStatics.GetGameMode`)))
  (for _array_element (`/Game/Blueprints/MapContent/BP_MapGrid.AllTiles` (`/Game/Blueprints/TileBasedGameMode.MapGridReference` _astile_based_game_mode))
    (bind _asbasic_tile (cast `/Game/Blueprints/MapContent/BasicTile` _array_element))
    (bind (_unit _isempty) (`/Game/Blueprints/MapContent/BasicTile.curUnitOrEmpty` _asbasic_tile))
    (bind _returnvalue (`|SpawnActorFromClass` "/Game/Blueprints/MapContent/Pathfinding/PathNode.PathNode_C" (`self.GetTransform` _array_element) "AlwaysSpawn" "OverrideRootScale"))
    (`/Game/Blueprints/MapContent/Pathfinding/PathNode.InstantiatePathNode` _returnvalue (`/Game/Blueprints/MapContent/BasicTile._X` _asbasic_tile) (`/Game/Blueprints/MapContent/BasicTile._Y` _asbasic_tile) (`/Game/Blueprints/MapContent/BasicTile.MovementCost` _asbasic_tile) _isempty)
    (`KismetArrayLibrary.Array_Add` (`self.PathGrid`) _returnvalue)))

(fn `findNodeAt`
  (params (X :type Integer) (Y :type Integer))
  (returns (`Array Element` :type "/Game/Blueprints/MapContent/Pathfinding/PathNode Object Reference"))
  (for _array_element (`self.PathGrid`)
    (if (and (== (`/Game/Blueprints/MapContent/Pathfinding/PathNode.X` _array_element) X) (== Y (`/Game/Blueprints/MapContent/Pathfinding/PathNode.Y` _array_element)))
      (return _array_element)))
  (return null))

(fn `FindTilesInRange`
  (params (Range :type Integer) (StartNode :type "/Game/Blueprints/MapContent/Pathfinding/PathNode Object Reference"))
  (bind _openset (`self.OpenSet`))
  (`KismetArrayLibrary.Array_Clear` (`self.ClosedSet`))
  (`KismetArrayLibrary.Array_Clear` _openset)
  (`KismetArrayLibrary.Array_Add` _openset StartNode)
  (while (`KismetArrayLibrary.Array_Contains` _openset (`KismetArrayLibrary.Array_Get` _openset (`KismetArrayLibrary.Array_LastIndex` _openset)))
    (bind _variable (`self.GetNodeWithLowestCost` (`self.OpenSet`))
      (:`Completed`
        (bind _array (`self.ValidNeighbours` _variable)
          (:`Completed`
            (for _ _array
              _)))))))

(fn `showPathNodes`
  (for _array_element (`self.PathGrid`)
    (bind _returnvalue (`AddComponent|NODE_AddStaticMeshComponent-0` :`self` _array_element))
    (`StaticMeshComponent.SetStaticMesh` _returnvalue "/Game/StarterContent/Props/MaterialSphere.MaterialSphere")))

(fn `updatePathfindingGrid`
  (bind _astile_based_game_mode (cast `/Game/Blueprints/TileBasedGameMode` (`GameplayStatics.GetGameMode`))
    (:`then`
      (for _array_element (`/Game/Blueprints/MapContent/BP_MapGrid.AllTiles` (`/Game/Blueprints/TileBasedGameMode.MapGridReference` _astile_based_game_mode))
        (bind _asbasic_tile (cast `/Game/Blueprints/MapContent/BasicTile` _array_element))
        (bind (_location_x _location_y _cost _occupied) (`/Game/Blueprints/MapContent/BasicTile.Information` _asbasic_tile))))
    (:`CastFailed`
      (`KismetSystemLibrary.PrintString` "UpdateGrid: Cast To TileBasedGameMode failed"))))

(fn `UserConstructionScript`)