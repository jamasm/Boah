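; Test player controller for a tile-based unit game, handling tile hover, tile selection and random unit spawning.
; Positive mouse movement triggers a cursor trace that stores the hovered BasicTile, which UpdateHUD returns with its path node.
; Pressing E spawns a shuffled unit type on a random empty tile.
; SelectTile swaps the selection, refreshes the pathfinding grid and, if occupied, arranges the unit's squads and requests its movement range from the game mode's pathfinder.
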(event `self.ReceiveBeginPlay`
  (bind _astile_based_game_mode (cast `/Game/Blueprints/TileBasedGameMode` (`GameplayStatics.GetGameMode`))
    (:`then`
      (set `self.TheGameMode` _astile_based_game_mode))
    (:`CastFailed`
      (`KismetSystemLibrary.PrintString` "wrong GameMode"))))

(event `Key|E`
  (params (Key :type "Key Structure" :default "AnyKey"))
  (:`Pressed`
    (`self.SpawnRandomUnit`)))

(event `self.ReceiveTick`
  (params (DeltaSeconds :type "Float (single-precision)"))
  (bind (_worldlocation _worlddirection) (`self.DeprojectMousePositionToWorld`))
  (bind (_deltax _deltay) (`self.GetInputMouseDelta`))
  (if (or (> _deltax 0.0) (> _deltay 0.0))
    (bind _outhits (`KismetSystemLibrary.LineTraceMulti` _worldlocation (+ _worldlocation (* _worlddirection 1000.0)) "TraceTypeQuery1"))
    (for _array_element _outhits
      (bind _asbasic_tile (cast `/Game/Blueprints/MapContent/BasicTile` (`.HitActor` (`GameplayStatics.BreakHitResult` _array_element))))
      (set `self.hover_Tile` _asbasic_tile))))

(fn `CallPathfinder`
  (params (StartTile :type "/Game/Blueprints/MapContent/BasicTile Object Reference"))
  (bind _pathfinderreference (`/Game/Blueprints/TileBasedGameMode.PathfinderReference` (`self.TheGameMode`)))
  (`/Game/Blueprints/MapContent/Pathfinding/Pathfinder.updatePathfindingGrid` _pathfinderreference)
  (`/Game/Blueprints/MapContent/Pathfinding/Pathfinder.UnitMovementRange` _pathfinderreference StartTile))

(fn `SelectTile`
  (params (Selected :type "/Game/Blueprints/MapContent/BasicTile Object Reference"))
  (bind _selectedtile (`self.SelectedTile`))
  (bind _item (`KismetArrayLibrary.Array_Get` (`self.SelectedTile`)))
  (for _array_element _selectedtile
    (`SceneComponent.ToggleVisibility` (`/Game/Blueprints/MapContent/BasicTile.SelectUI` _array_element) false))
  (`KismetArrayLibrary.Array_Clear` _selectedtile)
  (`KismetArrayLibrary.Array_Add` _selectedtile Selected)
  (`SceneComponent.ToggleVisibility` (`/Game/Blueprints/MapContent/BasicTile.SelectUI` Selected) false)
  (`/Game/Blueprints/MapContent/Pathfinding/Pathfinder.updatePathfindingGrid` (`/Game/Blueprints/TileBasedGameMode.PathfinderReference` (`self.TheGameMode`)))
  (bind (_unit _isempty) (`/Game/Blueprints/MapContent/BasicTile.curUnitOrEmpty` _item))
  (if (not _isempty)
    (`/Game/Blueprints/MapContent/BasicUnit.ArrangeSquads` _unit)
    (`self.CallPathfinder` _item)))

(fn `SpawnRandomUnit`
  (bind _thegamemode (`self.TheGameMode`))
  (bind _unittypes (`/Game/Blueprints/TileBasedGameMode.UnitTypes` _thegamemode))
  (bind _availabletiles (`/Game/Blueprints/MapContent/BP_MapGrid.getEmptyTiles` (`/Game/Blueprints/TileBasedGameMode.MapGridReference` _thegamemode)))
  (if (not (`/Engine/EditorBlueprintResources/StandardMacros.isArrayEmpty` _availabletiles))
    (`KismetArrayLibrary.Array_Shuffle` _availabletiles)
    (`KismetArrayLibrary.Array_Shuffle` _unittypes)
    (bind _item (`KismetArrayLibrary.Array_Get` _availabletiles))
    (bind _returnvalue (`|SpawnActorFromClass` (`KismetArrayLibrary.Array_Get` _unittypes (`KismetArrayLibrary.Array_LastIndex` _unittypes)) (`self.GetTransform` _item) "AlwaysSpawn" "OverrideRootScale"))
    (`/Game/Blueprints/MapContent/BasicTile.setUnit` _item _returnvalue)
    (bind (_unit _isempty) (`/Game/Blueprints/MapContent/BasicTile.curUnitOrEmpty` _item))
    (`KismetSystemLibrary.PrintString` (`KismetStringLibrary.Conv_BoolToString` _isempty) false)))

(fn `updateHUD`
  (returns (hover_Tile :type "/Game/Blueprints/MapContent/BasicTile Object Reference") (PathNode :type "/Game/Blueprints/MapContent/Pathfinding/PathNode Object Reference"))
  (bind _hover_tile (`self.hover_Tile`))
  (`KismetSystemLibrary.PrintString` (`KismetSystemLibrary.GetDisplayName` _hover_tile) true false)
  (bind (_location_x _location_y) (`/Game/Blueprints/MapContent/BasicTile.Information` (`self.hover_Tile`)))
  (bind _pathnode (`/Game/Blueprints/MapContent/Pathfinding/Pathfinder.findNodeAt` (`/Game/Blueprints/TileBasedGameMode.PathfinderReference` (`self.TheGameMode`)) _location_x _location_y))
  (return _hover_tile _pathnode))

(fn `UserConstructionScript`)